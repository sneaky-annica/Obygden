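; Base weapon Blueprint that fires projectiles on behalf of the Pawn that owns it.
; Fire compares game time against the last shot, so FireRate acts as the minimum seconds between shots, then calls SpawnProjectile.
; SpawnProjectile requires a Pawn owner and valid ProjectileClass, spawning at MuzzlePoint with owner and instigator set and passing on the weapon's Team.
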(fn `Fire`
  (if (>= (- (`KismetSystemLibrary.GetGameTimeInSeconds`) (`self.LastFireTime`)) (`self.FireRate`))
    (set `self.LastFireTime` (`KismetSystemLibrary.GetGameTimeInSeconds`))
    (`self.SpawnProjectile`)))

(fn `SpawnProjectile`
  (bind _aspawn (cast `Pawn` (`self.GetOwner`)))
  (bind _projectileclass (`self.ProjectileClass`)
    (:`then`
      (bind _returnvalue (`|SpawnActorFromClass` _projectileclass (`SceneComponent.K2_GetComponentToWorld` (`self.MuzzlePoint`)) "Undefined" "MultiplyWithRoot" (`self.GetOwner`) _aspawn))
      (set `/Game/Blueprints/Weapon/Projectile/BP_ProjectileBase.Team` (`self.Team`) _returnvalue))
    (:`else`)))

(fn `UserConstructionScript`)