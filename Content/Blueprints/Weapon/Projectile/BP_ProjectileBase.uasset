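; Base projectile actor for weapons that damages the first valid target it overlaps and then destroys itself.
; On BeginPlay it applies its Speed variable as the initial and max speed of its projectile movement component.
; Sphere overlaps skip the owner and ask actors implementing BPI_CanTakeDamage whether the projectile's Team can hurt them.
; Accepted targets receive an interface damage message with the damage and a target-to-projectile direction vector.
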(event `self.ReceiveBeginPlay`
  (bind _projectilemovementcomponent (`self.ProjectileMovementComponent`))
  (bind _output_get (set `ProjectileMovementComponent.InitialSpeed` (`self.Speed`) _projectilemovementcomponent))
  (set `ProjectileMovementComponent.MaxSpeed` _output_get _projectilemovementcomponent))

(event `self.SphereCollision.OnComponentBeginOverlap`
  (params (OverlappedComponent :type "PrimitiveComponent Object Reference") (OtherActor :type "Actor Object Reference") (OtherComp :type "PrimitiveComponent Object Reference") (OtherBodyIndex :type Integer) (bFromSweep :type Boolean) (SweepResult :type "HitResult Structure (by ref)"))
  (bind _isvalid (`self.IsValidTarget` OtherActor))
  (if _isvalid
    (`self.InflictDamage` OtherActor)
    (`self.K2_DestroyActor`)))

(fn `InflictDamage`
  (params (OtherActor :type "Actor Object Reference"))
  (message `/Game/Blueprints/Interfaces/BPI_CanTakeDamage.TakeDamage` OtherActor (`self.Damage`) (- (`self.K2_GetActorLocation`) (`self.K2_GetActorLocation` OtherActor))))

(fn `IsValidTarget`
  (params (OtherActor :type "Object Object Reference"))
  (returns (IsValid :type Boolean))
  (if (== OtherActor (`self.GetOwner`))
    _
    (elif (`KismetSystemLibrary.DoesImplementInterface` (`local.OtherActor`) "/Game/Blueprints/Interfaces/BPI_CanTakeDamage.BPI_CanTakeDamage_C")
      (bind _cantakedamage (message `/Game/Blueprints/Interfaces/BPI_CanTakeDamage.CanTakeDamageBy` (`local.OtherActor`) (`self.Team`)))
      (return _cantakedamage))))

(fn `UserConstructionScript`)