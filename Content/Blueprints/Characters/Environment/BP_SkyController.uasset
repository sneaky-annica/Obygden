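; BP_SkyController drives the day-night motion of the sun and moon from the game's clock.
; On BeginPlay it caches the GameState as a BP_TimeManager.
; Every Tick it converts current time over hours per day into an angle and sets the pitch of the SunOrbit component, offset by half a turn.
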(event `self.ReceiveBeginPlay`
  (bind _asbp_time_manager (cast `/Game/Blueprints/Game/BP_TimeManager` (`GameplayStatics.GetGameState`)))
  (set `self.TimeManager` _asbp_time_manager))

(event `self.ReceiveTick`
  (params (DeltaSeconds :type "Float (single-precision)"))
  (`self.RotateSunAndMoon`))

(fn `RotateSunAndMoon`
  (bind _timemanager (`self.TimeManager`)
    (:`then`
      (bind _output_get (set `self.SunAngle` (* (/ (`/Game/Blueprints/Game/BP_TimeManager.CurrentTime` _timemanager) (`/Game/Blueprints/Game/BP_TimeManager.HoursOnADay` _timemanager)) -360.0)))
      (`SceneComponent.K2_SetRelativeRotation` (`self.SunOrbit`) (`KismetMathLibrary.MakeRotator` 0.0 (- _output_get 180.0)) false false))
    (:`else`)))

(fn `UserConstructionScript`)