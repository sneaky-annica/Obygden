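; Base NPC Blueprint that keeps its AI Blackboard in sync with the day phase and can steer itself back toward world paths.
; On BeginPlay it gets the GameState's TimeManager, waiting for managers if needed, binds phase changes and caches BP_Path actors.
; RunPathCorrection, not called within this Blueprint, finds the nearest spline point and adds movement input along only the sideways offset when it exceeds MaxPathWidth.
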(event `RegisterToGameState`
  ;[0.2647 0.7865 0.01229 0.5] Register To GameState
  (bind _asbp_obygden_game_state (cast `/Game/Blueprints/Game/BP_Obygden_GameState` (`GameplayStatics.GetGameState`)))
  (bind _output_get (set `self.GameState` _asbp_obygden_game_state))
  (bind _timemanager (`/Game/Blueprints/Game/BP_Obygden_GameState.TimeManager` _output_get))
  (`/Engine/EditorBlueprintResources/StandardMacros.IsValid` _timemanager
    (:`Is Valid`
      (set `self.TimeManager` _timemanager)
      (`self.HandleBindOnDayPhaseChange`))
    (:`Is Not Valid`
      (add `/Game/Blueprints/Game/BP_Obygden_GameState.OnManagersReady` (`self.GameState`) (delegate `ManagersReady`)))))

(event `ManagersReady`
  ;[0.2647 0.7865 0.01229 0.5] Register To GameState
  (set `self.TimeManager` (`/Game/Blueprints/Game/BP_Obygden_GameState.TimeManager` (`self.GameState`)))
  (`self.HandleBindOnDayPhaseChange`))

(event `HandleBindOnDayPhaseChange`
  (add `/Game/Blueprints/Game/BP_DayTimeManager.OnDayPhaseChange` (`self.TimeManager`) (delegate `OnDayPhaseChange`)))

(event `OnDayPhaseChange`
  (params (Phase :type "/Game/Blueprints/Game/E_TimeOfDay Enum" :default "NewEnumerator0"))
  (`self.HandlePhaseChange` Phase))

(event `self.ReceiveBeginPlay`
  (`parent.ReceiveBeginPlay`)
  (`self.RegisterToGameState`)
  (`self.StoreBlackBoard`)
  (`self.SetDayPhase`)
  (`self.SetPaths`))

(fn `ApplyBestCorrection`
  (params (CurrentLocation :type "Vector Structure") (BestSpline :type "SplineComponent Object Reference") (BestPoint :type "Vector Structure"))
  (locals (ToSpline :type "Vector Structure") (SplineForward :type "Vector Structure") (ForwardComponent :type "Vector Structure") (SideVector :type "Vector Structure"))
  (bind _bestspline (`local.BestSpline`))
  (set `local.ToSpline` (- (`local.BestPoint`) (`local.CurrentLocation`)))
  (set `local.SplineForward` (`SplineComponent.GetDirectionAtSplineInputKey` _bestspline (`SplineComponent.FindInputKeyClosestToWorldLocation` _bestspline (`local.CurrentLocation`)) "World"))
  (set `local.ForwardComponent` (* (`KismetMathLibrary.Dot_VectorVector` (`local.ToSpline`) (`local.SplineForward`)) (`local.SplineForward`)))
  (bind _output_get (set `local.SideVector` (- (`local.ToSpline`) (`local.ForwardComponent`))))
  (if (> (`KismetMathLibrary.VSize` _output_get) (`self.MaxPathWidth`))
    (`self.AddMovementInput` (`KismetMathLibrary.Normal` (`local.SideVector`)) (`self.CorrectionStrength`))))

(fn `FindBestCorrection`
  (returns (CurrentLocation :type "Vector Structure") (BestSpline :type "SplineComponent Object Reference") (BestPoint :type "Vector Structure"))
  (locals (CurrentBestDistance :type "Float (double-precision)") (CurrentActorLocation :type "Vector Structure") (CurrentBestSpline :type "SplineComponent Object Reference") (CurrentBestPoint :type "Vector Structure"))
  (set `local.CurrentActorLocation` (`self.K2_GetActorLocation`))
  (set `local.CurrentBestDistance` 99999.0)
  (for _array_element _
    (bind _spline (`/Game/Blueprints/Environment/Path/BP_Path.Spline` _array_element))
    (bind _returnvalue (`SplineComponent.FindLocationClosestToWorldLocation` _spline (`local.CurrentActorLocation`) "World"))
    (bind _returnvalue_2 (`KismetMathLibrary.Vector_Distance` (`local.CurrentActorLocation`) _returnvalue))
    (if (< _returnvalue_2 (`local.CurrentBestDistance`))
      (set `local.CurrentBestDistance` _returnvalue_2)
      (set `local.CurrentBestSpline` _spline)
      (set `local.CurrentBestPoint` _returnvalue)))
  (return (`local.CurrentActorLocation`) (`local.CurrentBestSpline`) (`local.CurrentBestPoint`)))

(fn `HandlePhaseChange`
  (params (Phase :type "/Game/Blueprints/Game/E_TimeOfDay Enum" :default "NewEnumerator0"))
  (bind _blackboard (`self.BlackBoard`)
    (:`then`
      (`BlackboardComponent.SetValueAsEnum` _blackboard (`self.BBKey_DayPhase`) Phase))
    (:`else`)))

(fn `RunPathCorrection`
  (locals (BestPath :type " Structure" :default (struct :`CurrentLocation` (0.0 0.0 0.0) :`BestPoint` (0.0 0.0 0.0) :`BestDistance` 99999.0)))
  (bind (_currentlocation _bestspline _bestpoint) (`self.FindBestCorrection`))
  (`self.ApplyBestCorrection` _currentlocation _bestspline _bestpoint))

(fn `SetDayPhase`
  (bind _timemanager (`self.TimeManager`)
    (:`then`
      (`BlackboardComponent.SetValueAsEnum` (`self.BlackBoard`) (`self.BBKey_DayPhase`) (`/Game/Blueprints/Game/BP_DayTimeManager.CurrentPhase` _timemanager)))
    (:`else`)))

(fn `SetPaths`
  (bind _outactors (`GameplayStatics.GetAllActorsOfClass` "/Game/Blueprints/Environment/Path/BP_Path.BP_Path_C"))
  (set `self.Paths` _outactors))

(fn `StoreBlackBoard`
  (set `self.BlackBoard` (`AIBlueprintHelperLibrary.GetBlackboard` (`self.GetController`))))

(fn `UserConstructionScript`
  (`parent.UserConstructionScript`))