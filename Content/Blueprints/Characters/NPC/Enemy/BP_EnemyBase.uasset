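; Base enemy NPC that detects attackable targets, fights through AI and returns to its spawn point to despawn.
; A trigger sphere tracks enemy-destructible actors, while blackboard keys drive target-facing attacks, aggro and a new-day flag on phase change.
; CallForHelp alerts nearby enemies, which add the target and keep the higher aggro state.
; Stored spawn data routes enemies home via a branch teleporter when needed, where they destroy themselves and attached actors.
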(event `self.ReceiveBeginPlay`
  ;[0.42 0.7865 0.2428 0.5] Initialise
  (`parent.ReceiveBeginPlay`))

(event `self.TriggerSphere.OnComponentBeginOverlap`
  (params (OverlappedComponent :type "PrimitiveComponent Object Reference") (OtherActor :type "Actor Object Reference") (OtherComp :type "PrimitiveComponent Object Reference") (OtherBodyIndex :type Integer) (bFromSweep :type Boolean) (SweepResult :type "HitResult Structure (by ref)"))
  ;[0.42 0.7865 0.2428 0.5] Overlap Events
  (if (`KismetSystemLibrary.DoesImplementInterface` OtherActor "/Game/Blueprints/Interfaces/BPI_DestructableByEnemies.BPI_DestructableByEnemies_C")
    (`KismetArrayLibrary.Array_Add` (`self.DetectedActors`) OtherActor)))

(event `self.TriggerSphere.OnComponentEndOverlap`
  (params (OverlappedComponent :type "PrimitiveComponent Object Reference") (OtherActor :type "Actor Object Reference") (OtherComp :type "PrimitiveComponent Object Reference") (OtherBodyIndex :type Integer))
  ;[0.42 0.7865 0.2428 0.5] Overlap Events
  (if (`KismetSystemLibrary.DoesImplementInterface` OtherActor "/Game/Blueprints/Interfaces/BPI_DestructableByEnemies.BPI_DestructableByEnemies_C")
    (`KismetArrayLibrary.Array_RemoveItem` (`self.DetectedActors`) OtherActor)))

(event `/Game/Blueprints/Interfaces/BPI_Enemy.AnswerCallForHelp`
  (params (CombatTarget :type "Object Object Reference") (AggroState :type "/Game/Blueprints/AI/E_AggroState Enum" :default "NewEnumerator0"))
  ;[0.42 0.7865 0.2428 0.5] Combat
  (bind _asactor (cast `Actor` CombatTarget))
  (`KismetArrayLibrary.Array_AddUnique` (`self.DetectedActors`) _asactor)
  (`BlackboardComponent.SetValueAsEnum` (`self.BlackBoard`) (`self.BBKey_AggroState`) (`KismetMathLibrary.BMax` AggroState (`BlackboardComponent.GetValueAsEnum` (`self.BlackBoard`) (`self.BBKey_AggroState`)))))

(event `/Game/Blueprints/Interfaces/BPI_Enemy.AIAttack`
  ;[0.42 0.7865 0.2428 0.5] Combat
  (`self.RotateTowardsTarget`)
  (`self.Attack`))

(fn `CallForHelp`
  (params (AggroState :type "/Game/Blueprints/AI/E_AggroState Enum" :default "NewEnumerator0") (CombatTarget :type "Object Object Reference"))
  (locals (EnemyAllyBlackBoard :type "BlackboardComponent Object Reference"))
  (bind _outactors (`KismetSystemLibrary.SphereOverlapActors` (`self.K2_GetActorLocation`) 700.0 (`|MakeArray` "ObjectTypeQuery8" :!type "EObjectTypeQuery Enum") "BP_EnemyBase_C" (`|MakeArray` self :!type "Actor Object Reference")))
  (for _array_element _outactors
    (bind _asbp_enemy_base (cast `/Game/Blueprints/Characters/NPC/Enemy/BP_EnemyBase` _array_element))
    (`/Game/Blueprints/Interfaces/BPI_Enemy.AnswerCallForHelp` _asbp_enemy_base (`local.CombatTarget`) (`local.AggroState`))))

(fn `CanTakeDamageBy`
  (params (AttackTeam :type "/Game/Blueprints/Characters/E_TeamBelonging Enum" :default "NewEnumerator0"))
  (returns (CanTakeDamage :type Boolean))
  (return (`|EnumEquality` AttackTeam "NewEnumerator0")))

(fn `GetNextReturnLocation`
  (returns (NextLocation :type "Vector Structure"))
  (if (`self.HasSpawnedOnBranch`)
    (if (`self.IsCurrentlyOnBranch`)
      (return (`self.SpawnLocation`))
      (else
        (return (`SceneComponent.K2_GetComponentLocation` (`/Game/Blueprints/Environment/BranchTeleport/BP_EnemyBranchTeleport.MainInteractionBox` (`self.BranchTeleport`))))))
    (else
      (return (`self.SpawnLocation`)))))

(fn `HandleBackAtSpawnLocation`
  (for _array_element (`self.GetAttachedActors` true true)
    (`self.K2_DestroyActor` _array_element))
  (`self.K2_DestroyActor`))

(fn `HandlePhaseChange`
  (params (Phase :type "/Game/Blueprints/Game/E_TimeOfDay Enum" :default "NewEnumerator0"))
  (`parent.HandlePhaseChange` Phase)
  (if (`|EnumEquality` Phase "NewEnumerator0")
    (`BlackboardComponent.SetValueAsBool` (`self.BlackBoard`) (`self.BBKey_NewDayHasStarted`) true)))

(fn `HasTarget`
  (params (EnemyAlly :type "/Game/Blueprints/Characters/NPC/Enemy/BP_EnemyBase Object Reference"))
  (returns (HasTarget :type Boolean))
  (return (`KismetSystemLibrary.IsValid` (`BlackboardComponent.GetValueAsObject` (`AIBlueprintHelperLibrary.GetBlackboard` EnemyAlly) (`self.BBKey_CombatTarget`)))))

(fn `IsAlive`
  (returns (Alive :type Boolean))
  (return false))

(fn `RotateTowardsTarget`
  (bind _asactor (cast `Actor` (`BlackboardComponent.GetValueAsObject` (`self.BlackBoard`) (`self.BBKey_CombatTarget`))))
  (bind (_returnvalue_roll _returnvalue_pitch _returnvalue_yaw) (`KismetMathLibrary.BreakRotator` (`KismetMathLibrary.FindLookAtRotation` (`self.K2_GetActorLocation`) (`self.K2_GetActorLocation` _asactor))))
  (`self.K2_SetActorRotation` (`KismetMathLibrary.MakeRotator` 0.0 0.0 _returnvalue_yaw)))

(fn `StoreSpawnData`
  (params (SpawnGoundLocation :type "Vector Structure") (SpawnedOnBranch :type Boolean) (Teleporter :type "/Game/Blueprints/Environment/BranchTeleport/BP_EnemyBranchTeleport Object Reference"))
  (set `self.SpawnLocation` (`local.SpawnGoundLocation`))
  (`BlackboardComponent.SetValueAsVector` (`self.BlackBoard`) (`self.BBKey_SpawnLocation`) (`local.SpawnGoundLocation`))
  (bind _output_get (set `self.HasSpawnedOnBranch` (`local.SpawnedOnBranch`)))
  (set `self.IsCurrentlyOnBranch` _output_get)
  (set `self.BranchTeleport` (`local.Teleporter`)))

(fn `UserConstructionScript`)