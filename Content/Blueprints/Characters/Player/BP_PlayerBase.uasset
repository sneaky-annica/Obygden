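; Base player character that moves left and right along the world X axis from Enhanced Input.
; IA_Move first turns the mesh to face the sign of the current X acceleration, then feeds its value into movement input.
; Only the mesh's relative yaw flips between two opposite facings.
; EndPlay removes the input mapping context through CleanUp, while BeginPlay only calls the parent.
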(event `self.ReceiveBeginPlay`
  (`parent.ReceiveBeginPlay`))

(event `EnhancedInput|/Game/Assets/Input/IA_Move`
  (params (ActionValue :type "Float (double-precision)") (ElapsedSeconds :type "Float (double-precision)") (TriggeredSeconds :type "Float (double-precision)") (InputAction :type "InputAction Object Reference" :default "/Game/Assets/Input/IA_Move.IA_Move"))
  (:`Triggered`
    (`self.RotateCharacter`)
    (`self.AddMovementInput` (1.0 0.0 0.0) ActionValue)))

(event `self.ReceiveEndPlay`
  (params (EndPlayReason :type "EEndPlayReason Enum" :default "Destroyed"))
  ; Will this even run?
  (`self.CleanUp`))

(fn `CleanUp`
  (bind _asplayer_controller (cast `PlayerController` (`self.GetController`)))
  (`EnhancedInputSubsystemInterface.RemoveMappingContext` (pcsubsystem `EnhancedInputLocalPlayerSubsystem` _asplayer_controller) (`self.InputMappingContext`) (struct)))

(fn `RotateCharacter`
  (bind _charactermovement (`self.CharacterMovement`)
    (:`then`
      (bind _returnvalue_x (`KismetMathLibrary.BreakVector` (`CharacterMovementComponent.GetCurrentAcceleration` _charactermovement)))
      (`/Engine/EditorBlueprintResources/StandardMacros.CompareFloat` _returnvalue_x
        (:`>`
          (`SceneComponent.K2_SetRelativeRotation` (`self.Mesh`) (struct :`Yaw` -90.0) false false))
        (:`<`
          (`SceneComponent.K2_SetRelativeRotation` (`self.Mesh`) (struct :`Yaw` 90.0) false false))))
    (:`else`)))

(fn `UserConstructionScript`)