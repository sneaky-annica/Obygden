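; Base enemy Blueprint that feeds its AI blackboard with day phase from the GameState's TimeManager, aggro and spawn data.
; A trigger sphere tracks enemy-destructible actors, and calls for help share targets with nearby enemies, keeping the higher aggro state.
; Path correction steers it sideways toward the nearest BP_Path spline when it strays beyond the path width.
; Return helpers route it to spawn, via teleporter for branch spawns, and destroy it with attachments on arrival.
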(event `RegisterToGameState`
  ;[0.42 0.7865 0.2428 0.5] Initialise
  ;;[0.2647 0.7865 0.01229 0.5] Register To GameState
  (bind _asbp_obygden_game_state (cast `/Game/Blueprints/Game/BP_Obygden_GameState` (`GameplayStatics.GetGameState`)))
  (bind _output_get (set `self.GameState` _asbp_obygden_game_state))
  (bind _timemanager (`/Game/Blueprints/Game/BP_Obygden_GameState.TimeManager` _output_get))
  (`/Engine/EditorBlueprintResources/StandardMacros.IsValid` _timemanager
    (:`Is Valid`
      (set `self.TimeManager` _timemanager)
      (`self.HandleBindOnDayPhaseChange`))
    (:`Is Not Valid`
      (add `/Game/Blueprints/Game/BP_Obygden_GameState.OnManagersReady` (`self.GameState`) (delegate `ManagersReady`)))))

(event `ManagersReady`
  ;[0.42 0.7865 0.2428 0.5] Initialise
  ;;[0.2647 0.7865 0.01229 0.5] Register To GameState
  (set `self.TimeManager` (`/Game/Blueprints/Game/BP_Obygden_GameState.TimeManager` (`self.GameState`)))
  (`self.HandleBindOnDayPhaseChange`))

(event `HandleBindOnDayPhaseChange`
  ;[0.42 0.7865 0.2428 0.5] Initialise
  (add `/Game/Blueprints/Game/BP_DayTimeManager.OnDayPhaseChange` (`self.TimeManager`) (delegate `OnDayPhaseChange`)))

(event `OnDayPhaseChange`
  (params (Phase :type "/Game/Blueprints/Game/E_TimeOfDay Enum" :default "NewEnumerator0"))
  ;[0.42 0.7865 0.2428 0.5] Initialise
  (`self.HandlePhaseChange` Phase))

(event `self.ReceiveBeginPlay`
  ;[0.42 0.7865 0.2428 0.5] Initialise
  (`parent.ReceiveBeginPlay`)
  (`self.RegisterToGameState`)
  (`self.StoreBlackBoard`)
  (`self.SetDayPhase`)
  (`self.SetPaths`))

(event `self.TriggerSphere.OnComponentBeginOverlap`
  (params (OverlappedComponent :type "PrimitiveComponent Object Reference") (OtherActor :type "Actor Object Reference") (OtherComp :type "PrimitiveComponent Object Reference") (OtherBodyIndex :type Integer) (bFromSweep :type Boolean) (SweepResult :type "HitResult Structure (by ref)"))
  ;[0.42 0.7865 0.2428 0.5] Overlap Events
  (if (`KismetSystemLibrary.DoesImplementInterface` OtherActor "/Game/Blueprints/Interfaces/BPI_DestructableByEnemies.BPI_DestructableByEnemies_C")
    (`KismetArrayLibrary.Array_Add` (`self.DetectedActors`) OtherActor)))

(event `self.TriggerSphere.OnComponentEndOverlap`
  (params (OverlappedComponent :type "PrimitiveComponent Object Reference") (OtherActor :type "Actor Object Reference") (OtherComp :type "PrimitiveComponent Object Reference") (OtherBodyIndex :type Integer))
  ;[0.42 0.7865 0.2428 0.5] Overlap Events
  (if (`KismetSystemLibrary.DoesImplementInterface` OtherActor "/Game/Blueprints/Interfaces/BPI_DestructableByEnemies.BPI_DestructableByEnemies_C")
    (`KismetArrayLibrary.Array_RemoveItem` (`self.DetectedActors`) OtherActor)))

(event `/Game/Blueprints/Interfaces/BPI_Enemy.AnswerCallForHelp`
  (params (CombatTarget :type "Object Object Reference") (AggroState :type "/Game/Blueprints/AI/E_AggroState Enum" :default "NewEnumerator0"))
  ;[0.42 0.7865 0.2428 0.5] Combat
  (bind _asactor (cast `Actor` CombatTarget))
  (`KismetArrayLibrary.Array_AddUnique` (`self.DetectedActors`) _asactor)
  (`BlackboardComponent.SetValueAsEnum` (`self.BlackBoard`) (`self.BBKey_AggroState`) (`KismetMathLibrary.BMax` AggroState (`BlackboardComponent.GetValueAsEnum` (`self.BlackBoard`) (`self.BBKey_AggroState`)))))

(event `/Game/Blueprints/Interfaces/BPI_Enemy.AIAttack`
  ;[0.42 0.7865 0.2428 0.5] Combat
  (`self.RotateTowardsTarget`)
  (`self.Attack`))

(fn `ApplyBestCorrection`
  (params (CurrentLocation :type "Vector Structure") (BestSpline :type "SplineComponent Object Reference") (BestPoint :type "Vector Structure"))
  (locals (ToSpline :type "Vector Structure") (SplineForward :type "Vector Structure") (ForwardComponent :type "Vector Structure") (SideVector :type "Vector Structure"))
  (bind _bestspline (`local.BestSpline`))
  (set `local.ToSpline` (- (`local.BestPoint`) (`local.CurrentLocation`)))
  (set `local.SplineForward` (`SplineComponent.GetDirectionAtSplineInputKey` _bestspline (`SplineComponent.FindInputKeyClosestToWorldLocation` _bestspline (`local.CurrentLocation`)) "World"))
  (set `local.ForwardComponent` (* (`KismetMathLibrary.Dot_VectorVector` (`local.ToSpline`) (`local.SplineForward`)) (`local.SplineForward`)))
  (bind _output_get (set `local.SideVector` (- (`local.ToSpline`) (`local.ForwardComponent`))))
  (if (> (`KismetMathLibrary.VSize` _output_get) (`self.MaxPathWidth`))
    (`self.AddMovementInput` (`KismetMathLibrary.Normal` (`local.SideVector`)) (`self.CorrectionStrength`))))

(fn `CallForHelp`
  (params (AggroState :type "/Game/Blueprints/AI/E_AggroState Enum" :default "NewEnumerator0") (CombatTarget :type "Object Object Reference"))
  (locals (EnemyAllyBlackBoard :type "BlackboardComponent Object Reference"))
  (bind _outactors (`KismetSystemLibrary.SphereOverlapActors` (`self.K2_GetActorLocation`) 700.0 (`|MakeArray` "ObjectTypeQuery8" :!type "EObjectTypeQuery Enum") "BP_EnemyBase_C" (`|MakeArray` self :!type "Actor Object Reference")))
  (for _array_element _outactors
    (bind _asbp_enemy_base (cast `/Game/Blueprints/Characters/Enemy/BP_EnemyBase` _array_element))
    (`/Game/Blueprints/Interfaces/BPI_Enemy.AnswerCallForHelp` _asbp_enemy_base (`local.CombatTarget`) (`local.AggroState`))))

(fn `CanTakeDamageBy`
  (params (AttackTeam :type "/Game/Blueprints/Characters/E_TeamBelonging Enum" :default "NewEnumerator0"))
  (returns (CanTakeDamage :type Boolean))
  (return (`|EnumEquality` AttackTeam "NewEnumerator0")))

(fn `FindBestCorrection`
  (returns (CurrentLocation :type "Vector Structure") (BestSpline :type "SplineComponent Object Reference") (BestPoint :type "Vector Structure"))
  (locals (CurrentBestDistance :type "Float (double-precision)") (CurrentActorLocation :type "Vector Structure") (CurrentBestSpline :type "SplineComponent Object Reference") (CurrentBestPoint :type "Vector Structure"))
  (set `local.CurrentActorLocation` (`self.K2_GetActorLocation`))
  (set `local.CurrentBestDistance` 99999.0)
  (for _array_element (`self.Paths`)
    (bind _spline (`/Game/Blueprints/Environment/Path/BP_Path.Spline` _array_element))
    (bind _returnvalue (`SplineComponent.FindLocationClosestToWorldLocation` _spline (`local.CurrentActorLocation`) "World"))
    (bind _returnvalue_2 (`KismetMathLibrary.Vector_Distance` (`local.CurrentActorLocation`) _returnvalue))
    (if (< _returnvalue_2 (`local.CurrentBestDistance`))
      (set `local.CurrentBestDistance` _returnvalue_2)
      (set `local.CurrentBestSpline` _spline)
      (set `local.CurrentBestPoint` _returnvalue)))
  (return (`local.CurrentActorLocation`) (`local.CurrentBestSpline`) (`local.CurrentBestPoint`)))

(fn `GetNextReturnLocation`
  (returns (NextLocation :type "Vector Structure"))
  (if (`self.HasSpawnedOnBranch`)
    (if (`self.IsCurrentlyOnBranch`)
      (return (`self.SpawnLocation`))
      (else
        (return (`SceneComponent.K2_GetComponentLocation` (`/Game/Blueprints/Environment/BranchTeleport/BP_EnemyBranchTeleport.MainInteractionBox` (`self.BranchTeleport`))))))
    (else
      (return (`self.SpawnLocation`)))))

(fn `HandleBackAtSpawnLocation`
  (for _array_element (`self.GetAttachedActors` true true)
    (`self.K2_DestroyActor` _array_element))
  (`self.K2_DestroyActor`))

(fn `HandlePhaseChange`
  (params (Phase :type "/Game/Blueprints/Game/E_TimeOfDay Enum" :default "NewEnumerator0"))
  (bind _blackboard (`self.BlackBoard`)
    (:`then`
      (`BlackboardComponent.SetValueAsEnum` _blackboard (`self.BBKey_DayPhase`) Phase)
      (if (`|EnumEquality` Phase "NewEnumerator0")
        (`BlackboardComponent.SetValueAsBool` (`self.BlackBoard`) (`self.BBKey_NewDayHasStarted`) true)))
    (:`else`)))

(fn `HasTarget`
  (params (EnemyAlly :type "/Game/Blueprints/Characters/Enemy/BP_EnemyBase Object Reference"))
  (returns (HasTarget :type Boolean))
  (return (`KismetSystemLibrary.IsValid` (`BlackboardComponent.GetValueAsObject` (`AIBlueprintHelperLibrary.GetBlackboard` EnemyAlly) (`self.BBKey_CombatTarget`)))))

(fn `RotateTowardsTarget`
  (bind _blackboard (`self.BlackBoard`)
    (:`then`
      (bind _asactor (cast `Actor` (`BlackboardComponent.GetValueAsObject` _blackboard (`self.BBKey_CombatTarget`))))
      (bind (_returnvalue_roll _returnvalue_pitch _returnvalue_yaw) (`KismetMathLibrary.BreakRotator` (`KismetMathLibrary.FindLookAtRotation` (`self.K2_GetActorLocation`) (`self.K2_GetActorLocation` _asactor))))
      (`self.K2_SetActorRotation` (`KismetMathLibrary.MakeRotator` 0.0 0.0 _returnvalue_yaw)))
    (:`else`)))

(fn `RunPathCorrection`
  (locals (BestPath :type " Structure" :default (struct :`CurrentLocation` (0.0 0.0 0.0) :`BestPoint` (0.0 0.0 0.0) :`BestDistance` 99999.0)))
  (bind (_currentlocation _bestspline _bestpoint) (`self.FindBestCorrection`))
  (`self.ApplyBestCorrection` _currentlocation _bestspline _bestpoint))

(fn `SetDayPhase`
  (bind _timemanager (`self.TimeManager`)
    (:`then`
      (`BlackboardComponent.SetValueAsEnum` (`self.BlackBoard`) (`self.BBKey_DayPhase`) (`/Game/Blueprints/Game/BP_DayTimeManager.CurrentPhase` _timemanager)))
    (:`else`)))

(fn `SetPaths`
  (bind _outactors (`GameplayStatics.GetAllActorsOfClass` "/Game/Blueprints/Environment/Path/BP_Path.BP_Path_C"))
  (set `self.Paths` _outactors))

(fn `StoreBlackBoard`
  (set `self.BlackBoard` (`AIBlueprintHelperLibrary.GetBlackboard` (`self.GetController`))))

(fn `StoreSpawnData`
  (params (SpawnGoundLocation :type "Vector Structure") (SpawnedOnBranch :type Boolean) (Teleporter :type "/Game/Blueprints/Environment/BranchTeleport/BP_EnemyBranchTeleport Object Reference"))
  (`self.BlackBoard`
    (:`then`
      (set `self.SpawnLocation` (`local.SpawnGoundLocation`))
      (`BlackboardComponent.SetValueAsVector` (`self.BlackBoard`) (`self.BBKey_SpawnLocation`) (`local.SpawnGoundLocation`))
      (bind _output_get (set `self.HasSpawnedOnBranch` (`local.SpawnedOnBranch`)))
      (set `self.IsCurrentlyOnBranch` _output_get)
      (set `self.BranchTeleport` (`local.Teleporter`)))
    (:`else`)))

(fn `UserConstructionScript`)