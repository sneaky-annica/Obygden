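; Base character Blueprint that handles a team-assigned weapon, health, hit reactions and death, with left/right facing along X.
; BeginPlay spawns and socket-attaches the weapon, which Attack fires only while horizontally stationary.
; Damage clamps health, then plays random front or back montages chosen from projectile direction and facing; death destroys attached actors and sets a short lifespan.
; A separate event disables movement and enables locally controlled ragdoll physics; CanTakeDamageBy defaults to false.
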(event `self.ReceiveBeginPlay`
  (`self.SpawnDefaultWeapon`))

(event `/Game/Blueprints/Interfaces/BPI_CanTakeDamage.TakeDamage`
  (params (Damage :type "Float (double-precision)") (ProjectileDirection :type "Vector Structure"))
  ;[0.42 0.7865 0.2428 0.5] Take Damage
  (if (`|EnumEquality` (`self.LifeState`) "NewEnumerator4")
    (`self.DecrementHealth` Damage)
    (if (== (`self.CurrentHealth`) 0.0)
      (`self.HandleDeath` ProjectileDirection)
      (else
        (`self.HitReact` ProjectileDirection)))))

(event `InitialiseRagdoll`
  ;[0.42 0.7865 0.2428 0.5] Ragdoll
  (`self.RagdollEffect`))

(fn `Attack`
  (if (== (`KismetMathLibrary.VSizeXY` (`MovementComponent.Velocity` (`self.CharacterMovement`))) 0.0)
    (bind _equippedweapon (`self.EquippedWeapon`)
      (:`then`
        (`/Game/Blueprints/Weapon/BP_WeaponBase.Fire` _equippedweapon))
      (:`else`))))

(fn `CanTakeDamageBy`
  (params (AttackTeam :type "/Game/Blueprints/Characters/E_TeamBelonging Enum" :default "NewEnumerator0"))
  (returns (CanTakeDamage :type Boolean))
  (return false))

(fn `DecrementHealth`
  (params (Damage :type "Float (double-precision)"))
  (set `self.CurrentHealth` (`KismetMathLibrary.FClamp` (- (`self.CurrentHealth`) Damage) 0.0 (`self.MaxHealth`))))

(fn `EndLife`
  (set `self.LifeState` "NewEnumerator0")
  (for _array_element (`self.GetAttachedActors` true true)
    (`self.K2_DestroyActor` _array_element))
  (`self.SetLifeSpan` 3.0))

(fn `HandleDeath`
  (params (ProjectileDirection :type "Vector Structure"))
  (`self.PlayDeathAnim` ProjectileDirection)
  (`self.EndLife`))

(fn `HitReact`
  (params (ProjectileDirection :type "Vector Structure"))
  (`self.PlayAnimMontage` (`KismetArrayLibrary.Array_Random` (select `bool` (== (> ProjectileDirection_X 0.0) (`self.FacingRight`)) :`false` (`self.HitReactAnimBack`) :`true` (`self.HitReactAnimFront`)))))

(fn `IsAlive`
  (returns (Alive :type Boolean))
  (return (`|EnumEquality` (`self.LifeState`) "NewEnumerator4")))

(fn `PlayDeathAnim`
  (params (HitDirection :type "Vector Structure"))
  (`self.PlayAnimMontage` (`KismetArrayLibrary.Array_Random` (select `bool` (== (> HitDirection_X 0.0) (`self.FacingRight`)) :`false` (`self.DeathAnimBack`) :`true` (`self.DeathAnimFront`)))))

(fn `RagdollEffect`
  (`CharacterMovementComponent.DisableMovement` (`self.CharacterMovement`))
  (if (`self.IsLocallyControlled`)
    (`PrimitiveComponent.SetCollisionProfileName` (`self.Mesh`) "Ragdoll" true)
    (`SkeletalMeshComponent.SetAllBodiesBelowSimulatePhysics` (`self.Mesh`) (`self.RagdollBoneName`) true true)
    (`PrimitiveComponent.SetCollisionEnabled` (`self.CapsuleComponent`) "QueryOnly")))

(fn `SpawnDefaultWeapon`
  (bind _returnvalue (`|SpawnActorFromClass` (`self.WeaponClass`) (`self.GetTransform`) "Undefined" "MultiplyWithRoot" null null))
  (bind _asbp_weapon_base (cast `/Game/Blueprints/Weapon/BP_WeaponBase` _returnvalue))
  (bind _output_get (set `self.EquippedWeapon` _asbp_weapon_base))
  (`self.SetOwner` _output_get self)
  (set `/Game/Blueprints/Weapon/BP_WeaponBase.Team` (`self.Team`) (`self.EquippedWeapon`))
  (`self.K2_AttachToComponent` (`self.EquippedWeapon`) (`self.Mesh`) (`self.DrawnWeaponSocketName`) "SnapToTarget" "SnapToTarget" "KeepRelative" true))

(fn `UserConstructionScript`)