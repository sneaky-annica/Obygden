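; BP_EnemySpawnSite is a placed spawn point that releases a wave of BP_TallGrey enemies when the day cycle reaches a specific phase.
; On BeginPlay it waits for the game state's managers to be ready, then subscribes to the TimeManager's day phase change.
; The trigger phase sets a fixed spawn count, then a self-calling event spawns enemies at the actor's transform with short random delays between them.
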(event `RegisterToGameState`
  (bind _asbp_obygden_game_state (cast `/Game/Blueprints/Game/BP_Obygden_GameState` (`GameplayStatics.GetGameState`)))
  (bind _output_get (set `self.GameState` _asbp_obygden_game_state))
  (add `/Game/Blueprints/Game/BP_Obygden_GameState.OnManagersReady` _output_get (delegate `ManagersReady`)))

(event `ManagersReady`
  (bind _output_get (set `self.Time Manager` (`/Game/Blueprints/Game/BP_Obygden_GameState.TimeManager` (`self.GameState`))))
  (add `/Game/Blueprints/Game/BP_DayTimeManager.OnDayPhaseChange` _output_get (delegate `OnDayPhaseChange`)))

(event `OnDayPhaseChange`
  (params (Phase :type "/Game/Blueprints/Game/E_TimeOfDay Enum" :default "NewEnumerator0"))
  (if (`|EnumEquality` Phase "NewEnumerator3")
    (`self.CalculateNumberToSpawn`)
    (`self.SpawnEnemies`)))

(event `self.ReceiveBeginPlay`
  (`self.RegisterToGameState`))

(event `SpawnEnemies`
  (if (> (`self.RemainingToSpawn`) 0)
    (`|SpawnActorFromClass` "/Game/Blueprints/Characters/Enemy/BP_TallGrey.BP_TallGrey_C" (`self.GetTransform`) "Undefined" "MultiplyWithRoot" null null)
    (`/Engine/EditorBlueprintResources/StandardMacros.DecrementInt` (`self.RemainingToSpawn`)
      (:`  `
        (`KismetSystemLibrary.Delay` (`KismetMathLibrary.RandomFloatInRange` 0.05 0.15))
        (`self.SpawnEnemies`)))))

(fn `CalculateNumberToSpawn`
  (bind _output_get (set `self.NumberToSpawn` 10))
  (set `self.RemainingToSpawn` _output_get))

(fn `UserConstructionScript`)