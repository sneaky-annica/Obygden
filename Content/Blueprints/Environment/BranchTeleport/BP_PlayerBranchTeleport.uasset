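; BP_PlayerBranchTeleport is a two-way teleporter that moves the player between a main area and a branch.
; Overlapping the main box shows a hold-interact widget and registers the actor as the player's interactable through BPI_PlayerInteract.
; Interacting sends the player to the branch teleport point, passing a walk-to location as well.
; Overlapping the branch box returns the player to the main teleport point automatically, without interaction.
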(event `self.MainInteractionBox.OnComponentBeginOverlap`
  (params (OverlappedComponent :type "PrimitiveComponent Object Reference") (OtherActor :type "Actor Object Reference") (OtherComp :type "PrimitiveComponent Object Reference") (OtherBodyIndex :type Integer) (bFromSweep :type Boolean) (SweepResult :type "HitResult Structure (by ref)"))
  (if (`KismetSystemLibrary.DoesImplementInterface` OtherActor "/Game/Blueprints/Interfaces/Interactable/BPI_PlayerInteract.BPI_PlayerInteract_C")
    (`SceneComponent.SetVisibility` (`self.InteractionWidget`) true false)
    (message `/Game/Blueprints/Interfaces/Interactable/BPI_PlayerInteract.SetCurrentInteractable` OtherActor self)
    (message `/Game/Blueprints/Interfaces/Interactable/BPI_PlayerInteract.SetCurrentWidget` OtherActor (`self.InteractWidgetRef`))))

(event `self.MainInteractionBox.OnComponentEndOverlap`
  (params (OverlappedComponent :type "PrimitiveComponent Object Reference") (OtherActor :type "Actor Object Reference") (OtherComp :type "PrimitiveComponent Object Reference") (OtherBodyIndex :type Integer))
  (if (`KismetSystemLibrary.DoesImplementInterface` OtherActor "/Game/Blueprints/Interfaces/Interactable/BPI_PlayerInteract.BPI_PlayerInteract_C")
    (`SceneComponent.SetVisibility` (`self.InteractionWidget`) false false)
    (message `/Game/Blueprints/Interfaces/Interactable/BPI_PlayerInteract.SetCurrentInteractable` OtherActor null)))

(event `self.BranchInteractionBox.OnComponentBeginOverlap`
  (params (OverlappedComponent :type "PrimitiveComponent Object Reference") (OtherActor :type "Actor Object Reference") (OtherComp :type "PrimitiveComponent Object Reference") (OtherBodyIndex :type Integer) (bFromSweep :type Boolean) (SweepResult :type "HitResult Structure (by ref)"))
  (if (`KismetSystemLibrary.DoesImplementInterface` OtherActor "/Game/Blueprints/Interfaces/Interactable/BPI_PlayerInteract.BPI_PlayerInteract_C")
    (bind _asbp_player_base (cast `/Game/Blueprints/Characters/Player/BP_PlayerBase` OtherActor))
    (`/Game/Blueprints/Characters/Player/BP_PlayerBase.TeleportToMain` _asbp_player_base (`SceneComponent.K2_GetComponentLocation` (`self.MainTeleportPoint`)))))

(event `/Game/Blueprints/Interfaces/Interactable/BPI_Interactable.Interact`
  (params (Player :type "/Game/Blueprints/Characters/Player/BP_PlayerBase Object Reference"))
  (`/Game/Blueprints/Characters/Player/BP_PlayerBase.TeleportToBranch` Player (`SceneComponent.K2_GetComponentLocation` (`self.BranchTeleportPoint`)) (`SceneComponent.K2_GetComponentLocation` (`self.BranchWalkToPoint`))))

(event `self.ReceiveBeginPlay`
  (`self.SetInteractionWidget`))

(fn `SetInteractionWidget`
  (bind _aswbp_hold_interact (cast `/Game/Blueprints/UI/WBP_HoldInteract` (`WidgetComponent.GetUserWidgetObject` (`self.InteractionWidget`))))
  (set `self.InteractWidgetRef` _aswbp_hold_interact))

(fn `UserConstructionScript`)