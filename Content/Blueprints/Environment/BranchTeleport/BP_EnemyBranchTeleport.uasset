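; Environment actor that teleports enemies between a main area and a branch through two overlap boxes.
; Actors implementing BPI_Enemy that enter either box are sent to the teleport point on the opposite side.
; TeleportToLocation casts to BP_EnemyBase, stops AI movement, moves the enemy, updates its IsCurrentlyOnBranch flag, then restarts its brain logic so the AI re-evaluates from the new location.
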(event `self.BranchInteractionBox.OnComponentBeginOverlap`
  (params (OverlappedComponent :type "PrimitiveComponent Object Reference") (OtherActor :type "Actor Object Reference") (OtherComp :type "PrimitiveComponent Object Reference") (OtherBodyIndex :type Integer) (bFromSweep :type Boolean) (SweepResult :type "HitResult Structure (by ref)"))
  (if (`KismetSystemLibrary.DoesImplementInterface` OtherActor "/Game/Blueprints/Interfaces/BPI_Enemy.BPI_Enemy_C")
    (`self.TeleportToLocation` OtherActor (`SceneComponent.K2_GetComponentLocation` (`self.MainTeleportPoint`)))))

(event `self.MainInteractionBox.OnComponentBeginOverlap`
  (params (OverlappedComponent :type "PrimitiveComponent Object Reference") (OtherActor :type "Actor Object Reference") (OtherComp :type "PrimitiveComponent Object Reference") (OtherBodyIndex :type Integer) (bFromSweep :type Boolean) (SweepResult :type "HitResult Structure (by ref)"))
  (if (`KismetSystemLibrary.DoesImplementInterface` OtherActor "/Game/Blueprints/Interfaces/BPI_Enemy.BPI_Enemy_C")
    (`self.TeleportToLocation` OtherActor (`SceneComponent.K2_GetComponentLocation` (`self.BranchTeleportPoint`)) true)))

(fn `TeleportToLocation`
  (params (ControlledActor :type "Actor Object Reference") (TeleportLocation :type "Vector Structure") (GoingToABranch :type Boolean))
  (locals (EnemyToTeleport :type "/Game/Blueprints/Characters/NPC/Enemy/BP_EnemyBase Object Reference"))
  (bind _asbp_enemy_base (cast `/Game/Blueprints/Characters/NPC/Enemy/BP_EnemyBase` ControlledActor))
  (set `local.EnemyToTeleport` _asbp_enemy_base)
  (`Controller.StopMovement` (`AIBlueprintHelperLibrary.GetAIController` ControlledActor))
  (`self.K2_SetActorLocation` (`local.EnemyToTeleport`) TeleportLocation false true)
  (set `/Game/Blueprints/Characters/NPC/Enemy/BP_EnemyBase.IsCurrentlyOnBranch` (`local.GoingToABranch`) (`local.EnemyToTeleport`))
  (`BrainComponent.RestartLogic` (`AIController.BrainComponent` (`AIBlueprintHelperLibrary.GetAIController` (`local.EnemyToTeleport`)))))

(fn `UserConstructionScript`)