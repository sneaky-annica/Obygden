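; BP_EnemySpawnSite is an enemy spawn point that spawns waves of BP_TallGrey at its own transform, scaled to the current day count.
; On BeginPlay it waits for the game state's managers, then spawns a first wave and listens for TimeManager day phase changes.
; One specific phase recalculates the count and triggers another wave.
; SpawnEnemies calls itself after short random delays to stagger spawns until none remain.
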(event `RegisterToGameState`
  ;[0.42 0.7865 0.2428 0.5] Game state setup
  (bind _asbp_obygden_game_state (cast `/Game/Blueprints/Game/BP_Obygden_GameState` (`GameplayStatics.GetGameState`)))
  (bind _output_get (set `self.GameState` _asbp_obygden_game_state))
  (add `/Game/Blueprints/Game/BP_Obygden_GameState.OnManagersReady` _output_get (delegate `ManagersReady`)))

(event `ManagersReady`
  ;[0.42 0.7865 0.2428 0.5] Game state setup
  (bind _output_get (set `self.Time Manager` (`/Game/Blueprints/Game/BP_Obygden_GameState.TimeManager` (`self.GameState`))))
  (add `/Game/Blueprints/Game/BP_DayTimeManager.OnDayPhaseChange` _output_get (delegate `OnDayPhaseChange`))
  (`self.CalculateNumberToSpawn` (`/Game/Blueprints/Game/BP_DayTimeManager.DayCount` (`self.Time Manager`)))
  (`self.SpawnEnemies`))

(event `OnDayPhaseChange`
  (params (Phase :type "/Game/Blueprints/Game/E_TimeOfDay Enum" :default "NewEnumerator0"))
  ;[0.42 0.7865 0.2428 0.5] Game state setup
  (if (`|EnumEquality` Phase "NewEnumerator3")
    (`self.CalculateNumberToSpawn` (`/Game/Blueprints/Game/BP_DayTimeManager.DayCount` (`self.Time Manager`)))
    (`self.SpawnEnemies`)))

(event `self.ReceiveBeginPlay`
  (`self.RegisterToGameState`))

(event `SpawnEnemies`
  (if (> (`self.RemainingToSpawn`) 0)
    (`|SpawnActorFromClass` "/Game/Blueprints/Characters/Enemy/BP_TallGrey.BP_TallGrey_C" (`self.GetTransform`) "Undefined" "MultiplyWithRoot" null null)
    (`/Engine/EditorBlueprintResources/StandardMacros.DecrementInt` (`self.RemainingToSpawn`)
      (:`  `
        (`KismetSystemLibrary.Delay` (`KismetMathLibrary.RandomFloatInRange` 0.05 0.15))
        (`self.SpawnEnemies`)))))

(fn `CalculateNumberToSpawn`
  (params (DayCount :type Integer))
  (bind _output_get (set `self.NumberToSpawn` (* DayCount 2)))
  (set `self.RemainingToSpawn` _output_get))

(fn `UserConstructionScript`)