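; BP_BranchSign is an interactable sign that moves the player between a main area and a branch area.
; Overlapping the teleport box registers the sign as the player's current interactable, and Interact sends the player to the branch teleport point with a walk-to location.
; Overlapping the return box immediately teleports a BP_PlayerBase back to the main teleport point, without any interaction.
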(event `self.TeleportInteractionBox.OnComponentBeginOverlap`
  (params (OverlappedComponent :type "PrimitiveComponent Object Reference") (OtherActor :type "Actor Object Reference") (OtherComp :type "PrimitiveComponent Object Reference") (OtherBodyIndex :type Integer) (bFromSweep :type Boolean) (SweepResult :type "HitResult Structure (by ref)"))
  (if (`KismetSystemLibrary.DoesImplementInterface` OtherActor "/Game/Blueprints/Interfaces/BPI_PlayerInteract.BPI_PlayerInteract_C")
    (message `/Game/Blueprints/Interfaces/BPI_PlayerInteract.SetCurrentInteractable` OtherActor self)))

(event `self.TeleportInteractionBox.OnComponentEndOverlap`
  (params (OverlappedComponent :type "PrimitiveComponent Object Reference") (OtherActor :type "Actor Object Reference") (OtherComp :type "PrimitiveComponent Object Reference") (OtherBodyIndex :type Integer))
  (if (`KismetSystemLibrary.DoesImplementInterface` OtherActor "/Game/Blueprints/Interfaces/BPI_PlayerInteract.BPI_PlayerInteract_C")
    (message `/Game/Blueprints/Interfaces/BPI_PlayerInteract.SetCurrentInteractable` OtherActor null)))

(event `self.ReturnInteractionBox.OnComponentBeginOverlap`
  (params (OverlappedComponent :type "PrimitiveComponent Object Reference") (OtherActor :type "Actor Object Reference") (OtherComp :type "PrimitiveComponent Object Reference") (OtherBodyIndex :type Integer) (bFromSweep :type Boolean) (SweepResult :type "HitResult Structure (by ref)"))
  (if (`KismetSystemLibrary.DoesImplementInterface` OtherActor "/Game/Blueprints/Interfaces/BPI_PlayerInteract.BPI_PlayerInteract_C")
    (bind _asbp_player_base (cast `/Game/Blueprints/Characters/Player/BP_PlayerBase` OtherActor))
    (`/Game/Blueprints/Characters/Player/BP_PlayerBase.TeleportToMain` _asbp_player_base (`SceneComponent.K2_GetComponentLocation` (`self.MainTeleportPoint`)))))

(event `/Game/Blueprints/Interfaces/BPI_Interactable.Interact`
  (params (Player :type "/Game/Blueprints/Characters/Player/BP_PlayerBase Object Reference"))
  (`/Game/Blueprints/Characters/Player/BP_PlayerBase.TeleportToBranch` Player (`SceneComponent.K2_GetComponentLocation` (`self.BranchTeleportPoint`)) (`SceneComponent.K2_GetComponentLocation` (`self.BranchWalkToPoint`))))

(fn `UserConstructionScript`)