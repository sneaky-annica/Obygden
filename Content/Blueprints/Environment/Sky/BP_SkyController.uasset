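; BP_SkyController drives the day-night sky, moving and lighting the sun and moon from the game's TimeManager.
; It gets TimeManager once the GameState signals managers are ready, then updates sun, moon and skylight every Tick.
; Time becomes orbit angles, with the moon's arc scaled to night length, while curves set intensities and sun color.
; The night phase swaps sun and moon visibility, and the skylight recaptures every frame.
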(event `self.ReceiveBeginPlay`
  (bind _asbp_obygden_game_state (cast `/Game/Blueprints/Game/BP_Obygden_GameState` (`GameplayStatics.GetGameState`)))
  (bind _output_get (set `self.GameState` _asbp_obygden_game_state))
  (add `/Game/Blueprints/Game/BP_Obygden_GameState.OnManagersReady` _output_get (delegate `ManagersReady`)))

(event `ManagersReady`
  (set `self.TimeManager` (`/Game/Blueprints/Game/BP_Obygden_GameState.TimeManager` (`self.GameState`))))

(event `self.ReceiveTick`
  (params (DeltaSeconds :type "Float (single-precision)"))
  (`self.TimeManager`
    (:`then`
      (`self.UpdateSun`)
      (`self.UpdateMoon`)
      (`self.UpdateSkyLight`))
    (:`else`)))

(fn `RotateMoon`
  (bind _returnvalue (`KismetMathLibrary.MakeRotator` 0.0 (+ (* (`self.MoonAngle`) -1.0) (`self.SunAngleOffset`))))
  (`SceneComponent.K2_SetRelativeRotation` (`self.MoonOrbit`) _returnvalue false false)
  (`SceneComponent.K2_SetRelativeRotation` (`self.LightOrbit_Moon`) _returnvalue false false))

(fn `RotateSun`
  (bind _returnvalue (`KismetMathLibrary.MakeRotator` 0.0 (+ (* (`self.SunAngle`) -1.0) (`self.SunAngleOffset`))))
  (`SceneComponent.K2_SetRelativeRotation` (`self.SunOrbit`) _returnvalue false false)
  (`SceneComponent.K2_SetRelativeRotation` (`self.LightOrbit_Sun`) _returnvalue false false))

(fn `UpdateMoon`
  (`self.UpdateMoonTime`)
  (`self.UpdateMoonAngle`)
  (`self.RotateMoon`)
  (`self.UpdateMoonIntensity`))

(fn `UpdateMoonAngle`
  (set `self.MoonAngle` (* (/ (`self.MoonTime`) (`/Game/Blueprints/Game/BP_DayTimeManager.NightLength` (`self.TimeManager`))) 180.0)))

(fn `UpdateMoonIntensity`
  (`LightComponent.SetIntensity` (`self.DirectionalLight_Moon`) (`CurveFloat.GetFloatValue` (`self.Curve_MoonIntesity`) (`/Game/Blueprints/Game/BP_DayTimeManager.CurrentTime` (`self.TimeManager`))))
  (if (`|EnumEquality` (`/Game/Blueprints/Game/BP_DayTimeManager.CurrentPhase` (`self.TimeManager`)) "NewEnumerator3")
    (`SceneComponent.SetVisibility` (`self.MoonBillboard`) true false)
    (`SceneComponent.SetVisibility` (`self.DirectionalLight_Moon`) true false)
    (else
      (`SceneComponent.SetVisibility` (`self.MoonBillboard`) false false)
      (`SceneComponent.SetVisibility` (`self.DirectionalLight_Moon`) false false))))

(fn `UpdateMoonTime`
  (bind (_phasedata_phase _phasedata_starthour) (break `/Game/Blueprints/Game/ST_TimePhase` (`/Game/Blueprints/Game/BP_DayTimeManager.GetPhaseData` (`self.TimeManager`) "NewEnumerator3")))
  (bind (_phasedata_phase_2 _phasedata_starthour_2) (break `/Game/Blueprints/Game/ST_TimePhase` (`/Game/Blueprints/Game/BP_DayTimeManager.GetPhaseData` (`self.TimeManager`) "NewEnumerator3")))
  (bind (_phasedata_phase_3 _phasedata_starthour_3 _phasedata_endhour) (break `/Game/Blueprints/Game/ST_TimePhase` (`/Game/Blueprints/Game/BP_DayTimeManager.GetPhaseData` (`self.TimeManager`) "NewEnumerator3")))
  (if (>= (`/Game/Blueprints/Game/BP_DayTimeManager.CurrentTime` (`self.TimeManager`)) _phasedata_starthour_2)
    ; Before midnight
    (set `self.MoonTime` (- (`/Game/Blueprints/Game/BP_DayTimeManager.CurrentTime` (`self.TimeManager`)) _phasedata_starthour))
    (else
      ; After midnight
      (set `self.MoonTime` (+ (`/Game/Blueprints/Game/BP_DayTimeManager.CurrentTime` (`self.TimeManager`)) _phasedata_endhour)))))

(fn `UpdateSkyLight`
  (`SkyLightComponent.SetIntensity` (`SkyLight.LightComponent` (`self.SkyLightComponent`)) (`CurveFloat.GetFloatValue` (`self.Curve_SkyLightIntensity`) (`/Game/Blueprints/Game/BP_DayTimeManager.CurrentTime` (`self.TimeManager`))))
  (`SkyLightComponent.RecaptureSky` (`SkyLight.LightComponent` (`self.SkyLightComponent`))))

(fn `UpdateSun`
  (`self.UpdateSunAngle`)
  (`self.RotateSun`)
  (`self.UpdateSunIntensity`))

(fn `UpdateSunAngle`
  (set `self.SunAngle` (* (/ (- (`/Game/Blueprints/Game/BP_DayTimeManager.CurrentTime` (`self.TimeManager`)) 6.0) (`/Game/Blueprints/Game/BP_DayTimeManager.HoursOnADayNightCycle` (`self.TimeManager`))) 360.0)))

(fn `UpdateSunIntensity`
  (`LightComponent.SetIntensity` (`self.DirectionalLight_Sun`) (`CurveFloat.GetFloatValue` (`self.Curve_SunIntensity`) (`/Game/Blueprints/Game/BP_DayTimeManager.CurrentTime` (`self.TimeManager`))))
  (`LightComponent.SetLightColor` (`self.DirectionalLight_Sun`) (`CurveLinearColor.GetLinearColorValue` (`self.CurveSunColor`) (`/Game/Blueprints/Game/BP_DayTimeManager.CurrentTime` (`self.TimeManager`))) true)
  (if (`|EnumInequality` (`/Game/Blueprints/Game/BP_DayTimeManager.CurrentPhase` (`self.TimeManager`)) "NewEnumerator3")
    (`SceneComponent.SetVisibility` (`self.SunBillboard`) true false)
    (`SceneComponent.SetVisibility` (`self.DirectionalLight_Sun`) true false)
    (else
      (`SceneComponent.SetVisibility` (`self.SunBillboard`) false false)
      (`SceneComponent.SetVisibility` (`self.DirectionalLight_Sun`) false false))))

(fn `UserConstructionScript`)