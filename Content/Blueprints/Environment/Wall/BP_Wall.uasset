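; BP_Wall is a destructible wall actor that loses health when it takes damage and is removed from the level at zero.
; Its TakeDamage event ignores hits once dead, otherwise subtracts damage from Health clamped between zero and MaxHealth, then clears Alive and destroys the actor when Health runs out.
; IsAlive exposes the Alive flag, and the construction script is empty.
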(event `/Game/Blueprints/Interfaces/BPI_Damageable.TakeDamage`
  (params (Damage :type "Float (double-precision)") (ProjectileDirection :type "Vector Structure"))
  (if (`self.Alive`)
    (bind _output_get (set `self.Health` (`KismetMathLibrary.FClamp` (- (`self.Health`) Damage) 0.0 (`self.MaxHealth`))))
    (if (== _output_get 0.0)
      (set `self.Alive` false)
      (`self.K2_DestroyActor`))))

(fn `IsAlive`
  (returns (Alive :type Boolean))
  (return (`self.Alive`)))

(fn `UserConstructionScript`)