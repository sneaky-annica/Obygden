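; Behavior tree task that picks an attack position near the AI's current combat target.
; It reads the combat target actor from the blackboard and steps back 150 units from the target's location toward the controlled pawn.
; The resulting point is written to the attack location blackboard key, then the task finishes successfully.
; If the combat target fails the Actor cast, the task never calls FinishExecute.
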(event `self.ReceiveExecuteAI`
  (params (OwnerController :type "AIController Object Reference") (ControlledPawn :type "Pawn Object Reference"))
  (bind _output_get (set `self.BlackBoard` (`AIBlueprintHelperLibrary.GetBlackboard` OwnerController)))
  (bind _asactor (cast `Actor` (`BlackboardComponent.GetValueAsObject` _output_get (`self.BBKey_CombatTarget`))))
  (bind _returnvalue (`Actor.K2_GetActorLocation` _asactor))
  (`BlackboardComponent.SetValueAsVector` (`self.BlackBoard`) (`self.BBKey_AttackLocation`) (- _returnvalue (* (`KismetMathLibrary.Normal` (- _returnvalue (`Actor.K2_GetActorLocation` ControlledPawn))) 150.0)))
  (`self.FinishExecute` true))