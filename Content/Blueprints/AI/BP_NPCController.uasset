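; AI controller that runs each possessed BP_NPCBase's behavior tree and can nudge the NPC back toward nearby path splines.
; On possession it caches all BP_Path actors; StartPathCorrection and StopPathCorrection toggle a fast looping correction timer.
; Each tick of that timer finds the closest spline point and strips the along-spline component from the offset.
; Movement input is added sideways only when that offset exceeds MaxPathWidth, scaled by CorrectionStrength.
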(event `self.ReceivePossess`
  (params (PossessedPawn :type "Pawn Object Reference"))
  (bind _asbp_npcbase (cast `/Game/Blueprints/Characters/NPC/BP_NPCBase` PossessedPawn))
  (bind _output_get (set `self.PossessedNPC` _asbp_npcbase))
  (`self.RunBehaviorTree` (`/Game/Blueprints/Characters/NPC/BP_NPCBase.BTree` _output_get))
  (`self.SetPaths`))

(fn `ApplyBestCorrection`
  (params (CurrentLocation :type "Vector Structure") (BestSpline :type "SplineComponent Object Reference") (BestPoint :type "Vector Structure"))
  (locals (ToSpline :type "Vector Structure") (SplineForward :type "Vector Structure") (ForwardComponent :type "Vector Structure") (SideVector :type "Vector Structure"))
  (bind _bestspline (`local.BestSpline`))
  (set `local.ToSpline` (- (`local.BestPoint`) (`local.CurrentLocation`)))
  (set `local.SplineForward` (`SplineComponent.GetDirectionAtSplineInputKey` _bestspline (`SplineComponent.FindInputKeyClosestToWorldLocation` _bestspline (`local.CurrentLocation`)) "World"))
  (set `local.ForwardComponent` (* (`KismetMathLibrary.Dot_VectorVector` (`local.ToSpline`) (`local.SplineForward`)) (`local.SplineForward`)))
  (bind _output_get (set `local.SideVector` (- (`local.ToSpline`) (`local.ForwardComponent`))))
  (if (> (`KismetMathLibrary.VSize` _output_get) (`self.MaxPathWidth`))
    (`Pawn.AddMovementInput` (`self.PossessedNPC`) (`KismetMathLibrary.Normal` (`local.SideVector`)) (`self.CorrectionStrength`) false)))

(fn `FindBestCorrection`
  (returns (CurrentLocation :type "Vector Structure") (BestSpline :type "SplineComponent Object Reference") (BestPoint :type "Vector Structure"))
  (locals (CurrentBestDistance :type "Float (double-precision)") (CurrentActorLocation :type "Vector Structure") (CurrentBestSpline :type "SplineComponent Object Reference") (CurrentBestPoint :type "Vector Structure"))
  (set `local.CurrentActorLocation` (`self.K2_GetActorLocation` (`self.PossessedNPC`)))
  (set `local.CurrentBestDistance` 99999.0)
  (for _array_element (`self.Paths`)
    (bind _spline (`/Game/Blueprints/Environment/Path/BP_Path.Spline` _array_element))
    (bind _returnvalue (`SplineComponent.FindLocationClosestToWorldLocation` _spline (`local.CurrentActorLocation`) "World"))
    (bind _returnvalue_2 (`KismetMathLibrary.Vector_Distance` (`local.CurrentActorLocation`) _returnvalue))
    (if (< _returnvalue_2 (`local.CurrentBestDistance`))
      (set `local.CurrentBestDistance` _returnvalue_2)
      (set `local.CurrentBestSpline` _spline)
      (set `local.CurrentBestPoint` _returnvalue)))
  (return (`local.CurrentActorLocation`) (`local.CurrentBestSpline`) (`local.CurrentBestPoint`)))

(fn `RunPathCorrection`
  (locals (BestPath :type " Structure" :default (struct :`CurrentLocation` (0.0 0.0 0.0) :`BestPoint` (0.0 0.0 0.0) :`BestDistance` 99999.0)))
  (`self.PossessedNPC`
    (:`then`
      (bind (_currentlocation _bestspline _bestpoint) (`self.FindBestCorrection`))
      (`self.ApplyBestCorrection` _currentlocation _bestspline _bestpoint))
    (:`else`)))

(fn `SetPaths`
  (bind _outactors (`GameplayStatics.GetAllActorsOfClass` "/Game/Blueprints/Environment/Path/BP_Path.BP_Path_C"))
  (set `self.Paths` _outactors))

(fn `StartPathCorrection`
  (if (not (`KismetSystemLibrary.K2_IsTimerActiveHandle` (`self.PathCorrectionTimer`)))
    (bind _returnvalue (`KismetSystemLibrary.K2_SetTimer` null "RunPathCorrection" 0.05 true))
    (set `self.PathCorrectionTimer` _returnvalue)))

(fn `StopPathCorrection`
  (`KismetSystemLibrary.K2_ClearAndInvalidateTimerHandle` (`self.PathCorrectionTimer`)))

(fn `UserConstructionScript`)