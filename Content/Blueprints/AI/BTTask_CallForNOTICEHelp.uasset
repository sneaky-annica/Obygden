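; Behavior Tree task that makes an enemy call for help at the NOTICE level of aggro.
; On execution it casts the controlled pawn to BP_EnemyBase and sets a blackboard flag marking that the NOTICE help call has been made.
; It then calls the enemy's CallForHelp with the blackboard's combat target and a fixed aggro state, and finishes successfully.
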(event `self.ReceiveExecuteAI`
  (params (OwnerController :type "AIController Object Reference") (ControlledPawn :type "Pawn Object Reference"))
  (bind _asbp_enemy_base (cast `/Game/Blueprints/Characters/Enemy/BP_EnemyBase` ControlledPawn))
  (bind _output_get (set `self.EnemyRef` _asbp_enemy_base))
  (`BlackboardComponent.SetValueAsBool` (`AIBlueprintHelperLibrary.GetBlackboard` _output_get) (`self.BBKey_HasCalledForNOTICEHelp`) true)
  (`/Game/Blueprints/Characters/Enemy/BP_EnemyBase.CallForHelp` (`self.EnemyRef`) "NewEnumerator1" (`BlackboardComponent.GetValueAsObject` (`AIBlueprintHelperLibrary.GetBlackboard` (`self.EnemyRef`)) (`self.BBKey_CombatTarget`)))
  (`self.FinishExecute` true))