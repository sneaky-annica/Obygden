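; Behavior tree service that updates an AI's combat state on the Blackboard each tick.
; While a combat target exists, it compares target distance to attack, chase and notice ranges, setting the booleans for decorators and raising AggroState.
; Aggro only escalates during a fight, keeping chase and notice true once reached, while attack follows range.
; Losing the target or a new-day flag resets combat and sets ShouldReturn.
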(event `self.ReceiveTickAI`
  (params (OwnerController :type "AIController Object Reference") (ControlledPawn :type "Pawn Object Reference") (DeltaSeconds :type "Float (single-precision)"))
  (bind _output_get (set `self.BlackBoard` (`AIBlueprintHelperLibrary.GetBlackboard` ControlledPawn)))
  (if (`BlackboardComponent.GetValueAsBool` _output_get (`self.BBKey_NewDayHasStarted`))
    ;[0.42 0.7865 0.2428 0.5] Reset After Night
    (`self.ResetCombat`)
    (`BlackboardComponent.SetValueAsBool` (`self.BlackBoard`) (`self.BBKey_NewDayHasStarted`) false)
    (else
      (`/Engine/EditorBlueprintResources/StandardMacros.IsValid` (`BlackboardComponent.GetValueAsObject` (`self.BlackBoard`) (`self.BBKey_CombatTarget`))
        (:`Is Valid`
          ;[0.42 0.7865 0.2428 0.5] In a Fight
          (set `self.HasEnteredFight` true)
          (set `self.DistanceToCombatTarget` (`BlackboardComponent.GetValueAsFloat` (`self.BlackBoard`) (`self.BBKey_DistanceToTarget`)))
          (`self.SetAttackState`)
          (`self.SetChaseState`)
          (`self.SetNoticeState`))
        (:`Is Not Valid`
          ;[0.42 0.7865 0.2428 0.5] Has Left a Fight
          (if (`self.HasEnteredFight`)
            (`self.ResetCombat`)
            (set `self.HasEnteredFight` false)))))))

(fn `ResetCombat`
  (`BlackboardComponent.SetValueAsObject` (`self.BlackBoard`) (`self.BBKey_CombatTarget`) null)
  (`BlackboardComponent.SetValueAsFloat` (`self.BlackBoard`) (`self.BBKey_DistanceToTarget`) 9999.0)
  (`BlackboardComponent.SetValueAsEnum` (`self.BlackBoard`) (`self.BBKey_AggroState`) 0)
  (`self.ResetDecoratorBooleans`)
  (`BlackboardComponent.SetValueAsBool` (`self.BlackBoard`) (`self.BBKey_ShouldReturn`) true))

(fn `ResetCombatIfDawnStarted`
  (if (and (`|EnumEquality` (`self.PreviousPhase`) "NewEnumerator3") (`|EnumInequality` (cast `/Game/Blueprints/Game/E_TimeOfDay` (`BlackboardComponent.GetValueAsEnum` (`self.BlackBoard`) (`self.BBKey_DayPhase`))) "NewEnumerator3"))
    (`self.ResetCombat`)))

(fn `ResetDecoratorBooleans`
  (`BlackboardComponent.SetValueAsBool` (`self.BlackBoard`) (`self.BBKey_ShouldAttack`) false)
  (`BlackboardComponent.SetValueAsBool` (`self.BlackBoard`) (`self.BBKey_ShouldChase`) false)
  (`BlackboardComponent.SetValueAsBool` (`self.BlackBoard`) (`self.BBKey_ShouldNotice`) false)
  (`BlackboardComponent.SetValueAsBool` (`self.BlackBoard`) (`self.BBKey_IsHelping`) false)
  (`BlackboardComponent.SetValueAsBool` (`self.BlackBoard`) (`self.BBKey_HasCalledForNOTICEHelp`) false)
  (`BlackboardComponent.SetValueAsBool` (`self.BlackBoard`) (`self.BBKey_HasCalledForCHASEHelp`) false))

(fn `SetAttackState`
  (bind _returnvalue (`self.ShouldAttack`))
  (`BlackboardComponent.SetValueAsBool` (`self.BlackBoard`) (`self.BBKey_ShouldAttack`) _returnvalue)
  (if _returnvalue
    (`BlackboardComponent.SetValueAsEnum` (`self.BlackBoard`) (`self.BBKey_AggroState`) 3)))

(fn `SetChaseState`
  (bind _returnvalue (`self.ShouldChase`))
  (`BlackboardComponent.SetValueAsBool` (`self.BlackBoard`) (`self.BBKey_ShouldChase`) _returnvalue)
  (if _returnvalue
    (`BlackboardComponent.SetValueAsEnum` (`self.BlackBoard`) (`self.BBKey_AggroState`) (`KismetMathLibrary.BMax` (`BlackboardComponent.GetValueAsEnum` (`self.BlackBoard`) (`self.BBKey_AggroState`)) 2))))

(fn `SetNoticeState`
  (bind _returnvalue (`self.ShouldNotice`))
  (`BlackboardComponent.SetValueAsBool` (`self.BlackBoard`) (`self.BBKey_ShouldNotice`) _returnvalue)
  (if _returnvalue
    (`BlackboardComponent.SetValueAsEnum` (`self.BlackBoard`) (`self.BBKey_AggroState`) (`KismetMathLibrary.BMax` (`BlackboardComponent.GetValueAsEnum` (`self.BlackBoard`) (`self.BBKey_AggroState`)) 1))))

(fn `ShouldAttack`
  (returns (ReturnValue :type Boolean))
  (return (<= (`self.DistanceToCombatTarget`) (`self.AttackRange`))))

(fn `ShouldChase`
  (returns (ReturnValue :type Boolean))
  (return (or (and (<= (`self.DistanceToCombatTarget`) (`self.ChaseRange`)) (> (`self.DistanceToCombatTarget`) (`self.AttackRange`))) (>= (`BlackboardComponent.GetValueAsEnum` (`self.BlackBoard`) (`self.BBKey_AggroState`)) 2))))

(fn `ShouldNotice`
  (returns (ReturnValue :type Boolean))
  (return (or (and (<= (`self.DistanceToCombatTarget`) (`self.NoticeRange`)) (> (`self.DistanceToCombatTarget`) (`self.ChaseRange`))) (>= (`BlackboardComponent.GetValueAsEnum` (`self.BlackBoard`) (`self.BBKey_AggroState`)) 1))))

(fn `UpdateDayPhase`
  (set `self.PreviousPhase` (cast `/Game/Blueprints/Game/E_TimeOfDay` (`BlackboardComponent.GetValueAsEnum` (`self.BlackBoard`) (`self.BBKey_DayPhase`)))))