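; Behavior tree task that makes an enemy take one step toward its combat target.
; It reads the target actor from the blackboard and casts the pawn to BP_EnemyBase for its step length.
; It then issues an AI move to a point that far along the direction to the target, finishing successfully when the move finishes.
; Failed casts stop execution without finishing the task.
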(event `self.ReceiveExecuteAI`
  (params (OwnerController :type "AIController Object Reference") (ControlledPawn :type "Pawn Object Reference"))
  (bind _returnvalue (`Actor.K2_GetActorLocation` (`self.EnemyRef`)))
  (set `self.ControllerRef` OwnerController)
  (bind _asbp_enemy_base (cast `/Game/Blueprints/Characters/Enemy/BP_EnemyBase` ControlledPawn))
  (set `self.EnemyRef` _asbp_enemy_base)
  (bind _asactor (cast `Actor` (`BlackboardComponent.GetValueAsObject` (`AIBlueprintHelperLibrary.GetBlackboard` (`self.EnemyRef`)) (`self.BBKey_CombatTargetName`))))
  (set `self.CombatTargetRef` _asactor)
  (`AITask_MoveTo.AIMoveTo` (`self.ControllerRef`) (+ _returnvalue (* (`KismetMathLibrary.GetDirectionUnitVector` _returnvalue (`Actor.K2_GetActorLocation` (`self.CombatTargetRef`))) (`/Game/Blueprints/Characters/Enemy/BP_EnemyBase.StepLength` (`self.EnemyRef`)))) null
    (:`OnMoveFinished`
      (`self.FinishExecute` true))))