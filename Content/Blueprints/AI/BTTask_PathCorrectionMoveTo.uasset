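; Behavior tree task that moves an enemy pawn to a destination with path correction active on its BP_EnemyController.
; The destination is the enemy's next return location when the returning blackboard flag is set, otherwise the selected blackboard vector.
; Success or failure stops path correction and finishes the task, while abort only stops movement.
; The spawn-arrival check exists but is never run.
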(event `self.ReceiveExecuteAI`
  (params (OwnerController :type "AIController Object Reference") (ControlledPawn :type "Pawn Object Reference"))
  (`self.SetVariables` OwnerController ControlledPawn)
  (`/Game/Blueprints/AI/BP_EnemyController.StartPathCorrection` (`self.EnemyController`))
  (set `self.Destination` (`self.FetchDestination`))
  (`|AIMoveTo` (`self.ControlledEnemy`) (`self.Destination`) null (`self.AcceptanceRadius`)
    (:`OnSuccess`
      (`/Game/Blueprints/AI/BP_EnemyController.StopPathCorrection` (`self.EnemyController`))
      (`self.FinishExecute` true))
    (:`OnFail`
      (`/Game/Blueprints/AI/BP_EnemyController.StopPathCorrection` (`self.EnemyController`))
      (`self.FinishExecute` false))))

(event `self.ReceiveAbortAI`
  (params (OwnerController :type "AIController Object Reference") (ControlledPawn :type "Pawn Object Reference"))
  (`Controller.StopMovement` OwnerController))

(fn `CheckBackAtSpawnLocation`
  (if (<= (`KismetMathLibrary.Vector_Distance` (`Actor.K2_GetActorLocation` (`self.ControlledEnemy`)) (`/Game/Blueprints/Characters/NPC/Enemy/BP_EnemyBase.SpawnLocation` (`self.ControlledEnemy`))) (+ (`self.AcceptanceRadius`) 100.0))
    (`/Game/Blueprints/Characters/NPC/Enemy/BP_EnemyBase.HandleBackAtSpawnLocation` (`self.ControlledEnemy`))))

(fn `FetchDestination`
  (returns (ReturnValue :type "Vector Structure"))
  (return (select `bool` (`BlackboardComponent.GetValueAsBool` (`AIBlueprintHelperLibrary.GetBlackboard` (`self.ControlledEnemy`)) (`self.BBKey_IsReturning`)) :`false` (`BlackboardComponent.GetValueAsVector` (`AIBlueprintHelperLibrary.GetBlackboard` (`self.EnemyController`)) (`.SelectedKeyName` (break `BlackboardKeySelector` (`self.MoveToLocation`)))) :`true` (`self.Next Location`))))

(fn `SetVariables`
  (params (Controller :type "Object Object Reference") (Pawn :type "Pawn Object Reference"))
  (bind _asbp_enemy_controller (cast `/Game/Blueprints/AI/BP_EnemyController` Controller))
  (set `self.EnemyController` _asbp_enemy_controller)
  (bind _asbp_enemy_base (cast `/Game/Blueprints/Characters/NPC/Enemy/BP_EnemyBase` Pawn))
  (bind _output_get (set `self.ControlledEnemy` _asbp_enemy_base))
  (bind _nextlocation (`/Game/Blueprints/Characters/NPC/Enemy/BP_EnemyBase.GetNextReturnLocation` _output_get))
  (set `self.Next Location` _nextlocation))