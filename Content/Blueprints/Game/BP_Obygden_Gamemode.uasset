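; Game mode for Obygden that sets up optional local two-player play with a separate pawn class per player.
; On BeginPlay it creates a second local player when EnableMultiplayer is set.
; Overrides of ChoosePlayerStart and SpawnDefaultPawnFor identify player one as controller 0, giving it the first PlayerStart found and Player1, and any other the second and Player2.
; Start assignment relies on GetAllActorsOfClass order rather than tags.
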(event `self.ReceiveBeginPlay`
  (if (`self.EnableMultiplayer`)
    (`GameplayStatics.CreatePlayer` -1)))

(fn `ChoosePlayerStart`
  (params (Player :type "Controller Object Reference"))
  (returns (ReturnValue :type "Actor Object Reference"))
  (if (== Player (`GameplayStatics.GetPlayerController` 0))
    (bind _outactors (`GameplayStatics.GetAllActorsOfClass` "/Script/Engine.PlayerStart"))
    (return (`|GetArrayItem` _outactors))
    (else
      (bind _outactors_2 (`GameplayStatics.GetAllActorsOfClass` "/Script/Engine.PlayerStart"))
      (return (`|GetArrayItem` _outactors_2 1)))))

(fn `SpawnDefaultPawnFor`
  (params (NewPlayer :type "Controller Object Reference") (StartSpot :type "Actor Object Reference"))
  (returns (ReturnValue :type "Pawn Object Reference"))
  (locals (Player1 :type "Pawn Class Reference" :default "/Script/Engine.BlueprintGeneratedClass'/Game/Blueprints/Characters/Player/Ada/BP_Ada.BP_Ada_C'") (Player2 :type "Pawn Class Reference" :default "/Script/Engine.BlueprintGeneratedClass'/Game/Blueprints/Characters/Player/Walter/BP_Walter.BP_Walter_C'"))
  (bind _returnvalue (`|SpawnActorFromClass` (select `bool` (== NewPlayer (`GameplayStatics.GetPlayerController` 0)) :`false` (`local.Player2`) :`true` (`local.Player1`)) (`self.GetTransform` (`local.StartSpot`)) "Undefined" "MultiplyWithRoot" null null))
  (`Controller.Possess` (`local.NewPlayer`) null)
  (return _returnvalue))

(fn `UserConstructionScript`)