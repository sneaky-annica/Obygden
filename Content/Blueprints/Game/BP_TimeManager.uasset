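; BP_TimeManager runs the in-game clock, converting real seconds into game hours and tracking the current phase: Dawn, Day, Evening or Night.
; Tick advances and wraps CurrentTime, then looks up its phase in the TimePhases hour ranges, which can cross midnight.
; A phase change fires the matching event dispatcher once, and EndPlay unbinds all four.
; CalculateCurrentTime offers interval-based advancement but is not called in this graph.
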(event `self.ReceiveBeginPlay`
  (set `self.TimeScale` (/ (`self.HoursOnADay`) (`self.DayLengthSeconds`))))

(event `self.ReceiveTick`
  (params (DeltaSeconds :type "Float (single-precision)"))
  (bind _output_get (set `self.CurrentTime` (mod (+ (`self.CurrentTime`) (* DeltaSeconds (`self.TimeScale`))) (`self.HoursOnADay`))))
  (bind _phase (`self.GetPhaseFromTime` _output_get))
  (`self.BroadcastBasedOnPhase` _phase))

(event `self.ReceiveEndPlay`
  (params (EndPlayReason :type "EEndPlayReason Enum" :default "Destroyed"))
  (`self.UnbindEventDispatchers`))

(fn `BroadcastBasedOnPhase`
  (params (PhaseInput :type "/Game/Blueprints/Game/E_TimeOfDay Enum" :default "NewEnumerator0"))
  (if (`|EnumInequality` PhaseInput (`self.CurrentPhase`))
    (bind _output_get (set `self.CurrentPhase` (`local.PhaseInput`)))
    (switch `/Game/Blueprints/Game/E_TimeOfDay` _output_get
      (:`NewEnumerator0`
        (`self.OnDawnStarted`))
      (:`NewEnumerator1`
        (`self.OnDayStarted`))
      (:`NewEnumerator2`
        (`self.OnEveningStarted`))
      (:`NewEnumerator3`
        (`self.OnNightStarted`)))))

(fn `CalculateCurrentTime`
  (set `self.CurrentTime` (+ (`self.CurrentTime`) (* (`self.UpdateTimeInterval`) (`self.TimeScale`))))
  (if (> (`self.CurrentTime`) (`self.HoursOnADay`))
    (set `self.CurrentTime` (- (`self.CurrentTime`) (`self.HoursOnADay`)))))

(fn `GetPhaseFromTime`
  (params (CurrentTimeInput :type "Float (double-precision)"))
  (returns (Phase :type "/Game/Blueprints/Game/E_TimeOfDay Enum"))
  (locals (LocalStartHour :type "Float (double-precision)") (LocalEndHour :type "Float (double-precision)") (LocalPhase :type "/Game/Blueprints/Game/E_TimeOfDay Enum"))
  (for _array_element (`self.TimePhases`)
    (bind (_phase _starthour _endhour) (break `/Game/Blueprints/Game/ST_TimePhase` _array_element))
    (set `local.LocalPhase` _phase)
    (set `local.LocalStartHour` _starthour)
    (set `local.LocalEndHour` _endhour)
    (if (<= (`local.LocalStartHour`) (`local.LocalEndHour`))
      ; Dawn, Day and Evening phase
      (if (and (>= (`local.CurrentTimeInput`) (`local.LocalStartHour`)) (< (`local.CurrentTimeInput`) (`local.LocalEndHour`)))
        (return (`local.LocalPhase`)))
      (else
        ; Midnight phase
        (if (or (>= (`local.CurrentTimeInput`) (`local.LocalStartHour`)) (< (`local.CurrentTimeInput`) (`local.LocalEndHour`)))
          (return (`local.LocalPhase`)))))))

(fn `UnbindEventDispatchers`
  (clear `self.OnDayStarted`)
  (clear `self.OnNightStarted`)
  (clear `self.OnEveningStarted`)
  (clear `self.OnDawnStarted`))

(fn `UserConstructionScript`)