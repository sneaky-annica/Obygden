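; BP_WallManager builds BP_Wall actors, keeps a registry of them and tracks which one is the current outer wall.
; RequestBuildWall holds only a placeholder resource check before BuildWall spawns a wall, links it back to the manager and registers it.
; Registering or unregistering rescans the list for the wall with the greatest X location and broadcasts OuterWallHasChanged when that wall changes.
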(fn `BuildWall`
  (params (Location :type "Transform Structure"))
  (bind _returnvalue (`|SpawnActorFromClass` "/Game/Blueprints/Environment/Wall/BP_Wall.BP_Wall_C" Location "AdjustIfPossibleButDontSpawnIfColliding" "MultiplyWithRoot" null null))
  (`/Engine/EditorBlueprintResources/StandardMacros.IsValid` _returnvalue
    (:`Is Valid`
      (set `/Game/Blueprints/Environment/Wall/BP_Wall.WallManager` self _returnvalue)
      (`self.RegisterWall` _returnvalue))))

(fn `RegisterWall`
  (params (Wall :type "/Game/Blueprints/Environment/Wall/BP_Wall Object Reference"))
  (`KismetArrayLibrary.Array_AddUnique` (`self.Walls`) Wall)
  (`self.UpdateCurrentOuterWall`))

(fn `RequestBuildWall`
  (params (Position :type "Transform Structure"))
  (`KismetSystemLibrary.PrintString` "Should check resources etc.")
  (`self.BuildWall` Position))

(fn `UnregisterWall`
  (params (Wall :type "/Game/Blueprints/Environment/Wall/BP_Wall Object Reference"))
  (`KismetArrayLibrary.Array_RemoveItem` (`self.Walls`) Wall)
  (`self.UpdateCurrentOuterWall`))

(fn `UpdateCurrentOuterWall`
  (locals (WallArrayElement :type "/Game/Blueprints/Environment/Wall/BP_Wall Object Reference") (LoopOuterWall :type "/Game/Blueprints/Environment/Wall/BP_Wall Object Reference"))
  (bind _returnvalue_x (`KismetMathLibrary.BreakVector` (`self.K2_GetActorLocation` (`local.WallArrayElement`))))
  (bind _returnvalue_x_2 (`KismetMathLibrary.BreakVector` (`self.K2_GetActorLocation` (`local.LoopOuterWall`))))
  (set `local.LoopOuterWall` null)
  (for _array_element (`self.Walls`)
    (set `local.WallArrayElement` _array_element)
    (`local.LoopOuterWall`
      (:`then`
        (if (> _returnvalue_x _returnvalue_x_2)
          (set `local.LoopOuterWall` (`local.WallArrayElement`))))
      (:`else`
        (set `local.LoopOuterWall` (`local.WallArrayElement`)))))
  (if (!= (`self.CurrentOuterWall`) (`local.LoopOuterWall`))
    (bind _output_get (set `self.CurrentOuterWall` (`local.LoopOuterWall`)))
    (`self.OuterWallHasChanged` _output_get)))

(fn `UserConstructionScript`)