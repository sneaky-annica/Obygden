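; Day-night cycle manager that runs the in-game clock, tracks the current time phase and counts days.
; BeginPlay derives the time scale and day/night lengths from the cycle settings and TimePhases data.
; Tick advances the wrapped clock and looks up its phase, handling ranges that cross midnight.
; On a phase change it fires the OnDayPhaseChange dispatcher, and entering the first enum phase increments the day count.
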(event `self.ReceiveBeginPlay`
  (`self.StoreEssentialVariables`))

(event `self.ReceiveTick`
  (params (DeltaSeconds :type "Float (single-precision)"))
  (bind _currenttime (`self.SetCurrentTime` DeltaSeconds))
  (bind _phase (`self.GetPhaseFromTime` _currenttime))
  (`self.BroadcastBasedOnPhase` _phase)
  (if (`self.NewDayStarted`)
    (`self.UpdateDayCount`)))

(fn `BroadcastBasedOnPhase`
  (params (PhaseInput :type "/Game/Blueprints/Game/E_TimeOfDay Enum" :default "NewEnumerator0"))
  (if (`|EnumInequality` PhaseInput (`self.CurrentPhase`))
    (bind _output_get (set `self.CurrentPhase` (`local.PhaseInput`)))
    (`self.OnDayPhaseChange` _output_get)
    (set `self.NewDayStarted` (`|EnumEquality` (`self.CurrentPhase`) "NewEnumerator0"))))

(fn `GetPhaseData`
  (params (Phase :type "/Game/Blueprints/Game/E_TimeOfDay Enum" :default "NewEnumerator0"))
  (returns (PhaseData :type "/Game/Blueprints/Game/ST_TimePhase Structure"))
  (for _array_element (`self.TimePhases`)
    (if (`|EnumEquality` (`.Phase_2_670BE8064360E9CC9F5746BECEF41187` (break `/Game/Blueprints/Game/ST_TimePhase` _array_element)) Phase)
      (return _array_element))))

(fn `GetPhaseFromTime`
  (params (CurrentTimeInput :type "Float (double-precision)"))
  (returns (Phase :type "/Game/Blueprints/Game/E_TimeOfDay Enum"))
  (locals (LocalStartHour :type "Float (double-precision)") (LocalEndHour :type "Float (double-precision)") (LocalPhase :type "/Game/Blueprints/Game/E_TimeOfDay Enum"))
  (for _array_element (`self.TimePhases`)
    (bind (_phase _starthour _endhour) (break `/Game/Blueprints/Game/ST_TimePhase` _array_element))
    (set `local.LocalPhase` _phase)
    (set `local.LocalStartHour` _starthour)
    (set `local.LocalEndHour` _endhour)
    (if (<= (`local.LocalStartHour`) (`local.LocalEndHour`))
      ; Dawn, Day and Evening phase
      (if (and (>= (`local.CurrentTimeInput`) (`local.LocalStartHour`)) (< (`local.CurrentTimeInput`) (`local.LocalEndHour`)))
        (return (`local.LocalPhase`)))
      (else
        ; Midnight phase
        (if (or (>= (`local.CurrentTimeInput`) (`local.LocalStartHour`)) (< (`local.CurrentTimeInput`) (`local.LocalEndHour`)))
          (return (`local.LocalPhase`)))))))

(fn `SetCurrentTime`
  (params (DeltaSeconds :type "Float (double-precision)"))
  (returns (CurrentTime :type "Float (double-precision)"))
  (bind _output_get (set `self.CurrentTime` (mod (+ (`self.CurrentTime`) (* DeltaSeconds (`self.TimeScale`))) (`self.HoursOnADayNightCycle`))))
  (return _output_get))

(fn `StoreEssentialVariables`
  (bind (_phasedata_phase _phasedata_starthour) (break `/Game/Blueprints/Game/ST_TimePhase` (`self.GetPhaseData` "NewEnumerator0")))
  (bind (_phasedata_phase_2 _phasedata_starthour_2 _phasedata_endhour) (break `/Game/Blueprints/Game/ST_TimePhase` (`self.GetPhaseData` "NewEnumerator2")))
  (set `self.TimeScale` (/ (`self.HoursOnADayNightCycle`) (`self.DayNightPlaySeconds`)))
  (set `self.DayStart` _phasedata_starthour)
  (set `self.DayEnd` _phasedata_endhour)
  (set `self.DayLength` (- (`self.DayEnd`) (`self.DayStart`)))
  (set `self.NightLength` (- (`self.HoursOnADayNightCycle`) (`self.DayLength`))))

(fn `UpdateDayCount`
  (`/Engine/EditorBlueprintResources/StandardMacros.IncrementInt` (`self.DayCount`)
    (:`  `
      (set `self.NewDayStarted` false))))

(fn `UserConstructionScript`)